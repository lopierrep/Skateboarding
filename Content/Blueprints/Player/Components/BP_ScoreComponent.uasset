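; Player component that awards points for jumping over obstacles on a skateboard and shows the total in a WBP_Score widget.
; Owner capsule overlaps track actors with an ObstacleLogicComponent, and the skate movement component's jump event sets jump state.
; Leaving an obstacle adds its score value if the player is still airborne from a jump that began outside the overlap.
; Tick clears the jump flag once the character stops falling.
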(event Custom|OnPlayerBeginOverlap
  (params (OverlappedComponent :type Primitive%20Component%20Object%20Reference) (OtherActor :type Actor%20Object%20Reference) (OtherComp :type Primitive%20Component%20Object%20Reference) (OtherBodyIndex :type Integer) (bFromSweep :type Boolean) (SweepResult :type Hit%20Result%20Structure%20%28by%20ref%29))
  (Utilities|IsValid (Actor|GetComponentbyClass OtherActor "/Script/Skateboarding.ObstacleLogicComponent")
    (:Is%20Valid
      (Variables|Default|SetObstacle OtherActor)
      (Variables|Default|SetOverObstacle true)
      (Variables|Default|SetJumpCounter 0)
      (Variables|Default|SetValidPoint true))))

(event Custom|OnPlayerEndOverlap
  (params (OverlappedComponent :type Primitive%20Component%20Object%20Reference) (OtherActor :type Actor%20Object%20Reference) (OtherComp :type Primitive%20Component%20Object%20Reference) (OtherBodyIndex :type Integer))
  (bind _returnvalue (Actor|GetComponentbyClass OtherActor "/Script/Skateboarding.ObstacleLogicComponent"))
  (Utilities|IsValid _returnvalue
    (:Is%20Valid
      (if (== (Variables|Default|GetObstacle) OtherActor)
        (Variables|Default|SetOverObstacle false)
        (if (Math|Boolean|ANDBoolean (AI|Components|NavMovement|IsFalling (Variables|Default|GetCharacterMovement)) (== (Variables|Default|GetJumpCounter) 0) (Variables|Default|GetValidPoint) (Variables|Default|GetJumped)) :!label _label
          (Variables|Default|SetScore (+ (Variables|Default|GetScore) (Class|ObstacleLogicComponent|GetScoreValue _returnvalue)))
          (Variables|Default|SetJumpCounter 0)
          (Class|ScoreWidget|SetScore (Variables|Default|GetScoreWidget) (Utilities|String|ToString(Integer) (Variables|Default|GetScore))))
        (elif (AI|Components|NavMovement|IsFalling (Variables|Default|GetCharacterMovement))
          (goto _label))))))

(event Custom|OnJumped
  (Variables|Default|SetJumped true)
  (if (Variables|Default|GetOverObstacle)
    (Math|Integer|IncrementInt (Variables|Default|GetJumpCounter))))

(event EventBeginPlay
  (Utilities|FlowControl|Sequence
    (:then_0
      (Collision|BindEventtoOnComponentBeginOverlap (Actor|GetComponentbyClass (Components|GetOwner) "/Script/Engine.CapsuleComponent") (EventDispatchers|CreateEvent :!event Custom|OnPlayerBeginOverlap))
      (Collision|BindEventtoOnComponentEndOverlap (Actor|GetComponentbyClass (Components|GetOwner) "/Script/Engine.CapsuleComponent") (EventDispatchers|CreateEvent :!event Custom|OnPlayerEndOverlap)))
    (:then_1
      (EventDispatchers|BindEventtoOnJumped (Actor|GetComponentbyClass (Components|GetOwner) "/Game/Blueprints/Player/Components/BP_SkateMovementComponent.BP_SkateMovementComponent_C") (EventDispatchers|CreateEvent :!event Custom|OnJumped))
      (Variables|Default|SetSkateBack (Class|Actor|FindComponentbyTag (Variables|/Script/Engine.ChildActorComponent|GetChildActor (Class|Actor|FindComponentbyTag (Components|GetOwner) "/Script/Engine.ChildActorComponent" "skate")) "/Script/Engine.SceneComponent" "back"))
      (Variables|Default|SetCharacterMovement (Actor|GetComponentbyClass (Components|GetOwner) "/Script/Engine.CharacterMovementComponent"))
      (bind _returnvalue (UserInterface|CreateWidget "/Game/Blueprints/HUD/WBP_Score.WBP_Score_C"))
      (bind _output_get (Variables|Default|SetScoreWidget _returnvalue))
      (UserInterface|Viewport|AddtoViewport _output_get 0)
      (Class|ScoreWidget|SetScore (Variables|Default|GetScoreWidget) (Utilities|String|ToString(Integer) (Variables|Default|GetScore))))))

(event EventTick
  (params (DeltaSeconds :type Float%20%28single-precision%29))
  (|CallParentFunction DeltaSeconds)
  (if (Variables|Default|GetJumped)
    (if (AI|Components|NavMovement|IsFalling (Variables|Default|GetCharacterMovement))
      (if (and (Variables|Default|GetOverObstacle) (Variables|Default|GetValidPoint))
        (Variables|Default|SetValidPoint (AI|Components|NavMovement|IsFalling (Variables|Default|GetCharacterMovement))))
      (else
        (Variables|Default|SetJumped false)))))